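; Menu game mode that registers players joining the Lobby Menu level and shares their profiles among the connected players.
; On each new player start in that level, it stores the Menu_Player_Controller and tells it to create the lobby and load.
; UpdateLobby rebuilds the profile list from every stored controller, then passes the full list back to each one to update player names.
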(event Custom|UpdateLobby
  (Utilities|Array|Clear (Variables|Default|GetPlayerProfiles))
  (for _array_element (Variables|Default|GetAllConnectedPlayers)
    (Utilities|Array|Add (Variables|Default|GetPlayerProfiles) (Variables|/Game/Characters/Menu_Player_Controller.Menu_Player_Controller_C|GetPlayer%20Profile%20Struct _array_element)))
  (for _array_element_2 (Variables|Default|GetAllConnectedPlayers)
    (Default|UpdatePlayerName _array_element_2 (Variables|Default|GetPlayerProfiles))))

(event EventBeginPlay)

(event EventTick
  (params (DeltaSeconds :type Float%20%28single-precision%29)))

(event EventHandleStartingNewPlayer
  (params (NewPlayer :type Player%20Controller%20Object%20Reference))
  (bind _returnvalue (Game|GetCurrentLevelName true))
  (switch string _returnvalue
    (:Lobby_Menu
      (bind _asmenu_player_controller (Utilities|Casting|CastToMenu_Player_Controller NewPlayer))
      (Utilities|Array|Add (Variables|Default|GetAllConnectedPlayers) _asmenu_player_controller)
      (Default|CreateLobby _asmenu_player_controller)
      (Default|Load _asmenu_player_controller))))

(fn ConstructionScript)