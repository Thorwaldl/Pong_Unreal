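; Pong game mode that spawns the ball at match start and keeps both players' scores.
; NewBall spawns a Ball just above the origin with a random yaw in a 90-degree arc, flipped 180 degrees by its Condition, and prints a debug angle.
; The score functions increment a player's score and call CheckWin, which is still empty.
; An impulse launch on the ball's Sphere is left unconnected.
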(event EventBeginPlay
  (CallFunction|NewBall false))

(event EventTick
  (params (DeltaSeconds :type Float%20%28single-precision%29)))

(fn ConstructionScript)

(fn NewBall
  (params (Condition :type Boolean))
  (if Condition
    (Variables|Default|SetBallAngle 180)
    (else
      (Variables|Default|SetBallAngle 0)))
  (Development|PrintString (Utilities|String|ToString(Float) (Math|Conversions|ToFloat(Integer) (+ (+ (Class|KismetMathLibrary|RandomInteger64 90) 45) (Variables|Default|GetBallAngle)))))
  (bind _returnvalue (Game|SpawnActorfromClass "/Game/Ball.Ball_C" (Math|Transform|MakeTransform (Math|Vector|MakeVector 0.0 0.0 25.0) (Math|Rotator|MakeRotator 0.0 0.0 (Math|Conversions|ToFloat(Integer) (+ (+ (Class|KismetMathLibrary|RandomInteger64 90) 45) (Variables|Default|GetBallAngle))))) "Undefined" "MultiplyWithRoot" 0 0)))

(fn AddPlayer1Score
  (Variables|Default|SetPlayer1Score (+ 1 (Variables|Default|GetPlayer1Score)))
  (CallFunction|CheckWin))

(fn AddPlayer2Score
  (Variables|Default|SetPlayer2Score (+ 1 (Variables|Default|GetPlayer2Score)))
  (CallFunction|CheckWin))

(fn CheckWin)